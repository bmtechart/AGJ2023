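; Main game mode for what appears to be a submarine game, deciding when the match is won or lost.
; It starts the submarine music track on BeginPlay.
; Each tick it checks depth and water level against fixed thresholds, calling GameOver as a victory for depth and a defeat for water.
; GameOver has no logic in this graph, and nothing stops it being called again on later ticks.
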(event `self.ReceiveBeginPlay`
  ;[1 1 1] Start Music
  (`GameplayStatics.PlaySound2D` "/Game/Audio/Music/MUSIC_SubmarineLong.MUSIC_SubmarineLong" 0.5 1.0 0.0 null null))

(event `self.ReceiveTick`
  (params (DeltaSeconds :type "Float (single-precision)"))
  (`|ExecutionSequence`
    (:`then_0`
      (if (>= (`self.CurrentDepth`) 1.0)
        (`self.GameOver` true)))
    (:`then_1`
      (if (>= (`self.WaterLevel`) 0.0)
        (`self.GameOver` false)))))

(event `GameOver`
  (params (bVictory :type Boolean)))

(fn `UserConstructionScript`)