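; Repair task where the player turns a wrench with the mouse to fix a breakage, built on a parent task with Break, Fix and EnterTask events.
; Entering points the equipped tool at ToolSocket and shows a grab cursor; IA_Wrench input rotates the socket and accumulates rotation.
; Mouse deltas are adjusted by cursor position around the viewport center, approximating circular dragging.
; Break starts a Niagara effect that shrinks with progress; releasing at full rotation fixes and exits.
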(event `self.ReceiveTick`
  (params (DeltaSeconds :type "Float (single-precision)"))
  (bind _returnvalue (`KismetMathLibrary.FClamp` (- 1.0 (`KismetMathLibrary.NormalizeToRange` (`self.DeltaRotation`) 0.0 (`self.TotalRotationRequired`)))))
  (`parent.ReceiveTick` DeltaSeconds)
  (`SceneComponent.SetWorldScale3D` (`self.Niagara`) (`KismetMathLibrary.MakeVector` _returnvalue _returnvalue _returnvalue)))

(event `EnhancedInput|/Game/Input/Wrenching/IA_Wrench`
  (params (ActionValue :type Boolean) (ElapsedSeconds :type "Float (double-precision)") (TriggeredSeconds :type "Float (double-precision)") (InputAction :type "InputAction Object Reference" :default "/Game/Input/Wrenching/IA_Wrench.IA_Wrench"))
  (bind _returnvalue (`self.GetAdjustedRotationFromCursorAlpha`))
  (:`Triggered`
    (`SceneComponent.K2_AddRelativeRotation` (`self.ToolSocket`) (`KismetMathLibrary.MakeRotator` _returnvalue) false false)
    (set `self.DeltaRotation` (+ (`self.DeltaRotation`) _returnvalue)))
  (:`Completed`
    (if (>= (`KismetMathLibrary.NormalizeToRange` (`self.DeltaRotation`) 0.0 (`self.TotalRotationRequired`)) 1.0)
      (`self.Fix`)
      (`self.ExitTask`))))

(event `self.EnterTask`
  (bind _returnvalue (`GameplayStatics.GetPlayerController` 0))
  (set `/Game/Blueprints/Tools/BP_Tool.TargetSceneComponent` (`self.ToolSocket`) (`/Game/Blueprints/BP_Character.EquippedTool` (`self.Character Ref`)))
  (`PlayerController.SetMouseCursorWidget` _returnvalue "GrabHand" null)
  (set `PlayerController.bShowMouseCursor` true _returnvalue)
  (`parent.EnterTask`)
  (`GameplayStatics.SetViewportMouseCaptureMode` "CaptureDuringMouseDown"))

(event `self.Break`
  (`parent.Break`)
  (`ActorComponent.Activate` (`self.Niagara`) false)
  (`SceneComponent.SetWorldScale3D` (`self.Niagara`) (1.0 1.0 1.0))
  (set `self.DeltaRotation` 0.0))

(event `self.Fix`
  (`parent.Fix`)
  (`ActorComponent.Deactivate` (`self.Niagara`)))

(fn `GetAdjustedRotationFromCursorAlpha`
  (returns (ReturnValue :type "Float (double-precision)"))
  (locals (ViewportXMidpoint :type "Float (double-precision)") (ViewportYMidpoint :type "Float (double-precision)") (DeltaX :type "Float (single-precision)" :default 0.0) (DeltaY :type "Float (single-precision)" :default 0.0) (MousePosX :type "Float (double-precision)" :default 0.0) (MousePosY :type "Float (double-precision)" :default 0.0))
  (bind (_returnvalue_x _returnvalue_y) (`KismetMathLibrary.BreakVector2D` (`WidgetLayoutLibrary.GetViewportSize`)))
  (bind (_deltax _deltay) (`PlayerController.GetInputMouseDelta` (`GameplayStatics.GetPlayerController` 0)))
  (set `local.ViewportXMidpoint` (/ _returnvalue_x 2.0))
  (set `local.ViewportYMidpoint` (/ _returnvalue_y 2.0))
  (set `local.DeltaX` _deltax)
  (set `local.DeltaY` _deltay)
  (bind _returnvalue (`WidgetLayoutLibrary.GetMousePositionOnViewport`))
  (set `local.MousePosX` (`KismetMathLibrary.BreakVector2D` _returnvalue))
  (set `local.MousePosY` (`.Y` (`KismetMathLibrary.BreakVector2D` _returnvalue)))
  (`|ExecutionSequence`
    (:`then_0`
      (if (>= (`local.MousePosX`) (`local.ViewportXMidpoint`))
        (`/Engine/EditorBlueprintResources/StandardMacros.NegateFloat` (`local.DeltaY`))))
    (:`then_1`
      (if (>= (`local.MousePosY`) (`local.ViewportYMidpoint`))
        (`/Engine/EditorBlueprintResources/StandardMacros.NegateFloat` (`local.DeltaX`))))
    (:`then_2`
      (return (+ (`local.DeltaX`) (`local.DeltaY`))))))

(fn `UserConstructionScript`
  (`parent.UserConstructionScript`))