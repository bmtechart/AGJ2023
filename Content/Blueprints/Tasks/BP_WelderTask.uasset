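; Welding repair task where the player holds the weld input with a BP_Welder tool to seal a crack.
; Break shows the large crack and activates Niagara effects, while Fix deactivates them.
; Each weld press restarts the timer, which moves the tool socket along the WeldLine spline with camera rotation.
; Progress thresholds swap in smaller crack meshes, then hide the crack, call Fix and exit the task, stopping welder and sound.
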(event `self.Fix`
  (`parent.Fix`)
  (`ActorComponent.Deactivate` (`self.Niagara`)))

(event `self.Break`
  (bind _crackstate (`self.CrackState`))
  (`parent.Break`)
  (`ActorComponent.Activate` (`self.Niagara`) false)
  (`SceneComponent.SetVisibility` _crackstate true false)
  (`StaticMeshComponent.SetStaticMesh` _crackstate (`self.CrackStateLarge`)))

(event `EnhancedInput|/Game/Input/Welding/IA_Weld`
  (params (ActionValue :type Boolean) (ElapsedSeconds :type "Float (double-precision)") (TriggeredSeconds :type "Float (double-precision)") (InputAction :type "InputAction Object Reference" :default "/Game/Input/Welding/IA_Weld.IA_Weld"))
  (bind _weldline (`self.WeldLine`))
  (bind _equippedtool (`/Game/Blueprints/BP_Character.EquippedTool` (`self.Character Ref`)))
  (:`Triggered`
    (set `self.CurrentWeldTime` (+ (`self.CurrentWeldTime`) (`GameplayStatics.GetWorldDeltaSeconds`)))
    (`|ExecutionSequence`
      (:`then_0`
        ;[1 1 1] Move tool along spline
        (`SceneComponent.K2_SetWorldLocation` (`self.ToolSocket`) (`SplineComponent.GetLocationAtDistanceAlongSpline` _weldline (* (`SplineComponent.GetSplineLength` _weldline) (`KismetMathLibrary.NormalizeToRange` (`self.CurrentWeldTime`) 0.0 (`self.TargetWeldTime`))) "World") false false)
        (`SceneComponent.K2_SetWorldRotation` (`self.ToolSocket`) (`SceneComponent.K2_GetComponentRotation` (`self.Camera`)) false false))
      (:`then_1`
        ;[1 1 1] replace static meshes
        (switch `int` (`self.WeldState`)
          (:`0`
            ;;[1 1 1] Large to Medium
            (if (>= (`self.CurrentWeldTime`) (* (`self.TargetWeldTime`) 0.33))
              (`StaticMeshComponent.SetStaticMesh` (`self.CrackState`) (`self.CrackStateMedium`))
              (`/Engine/EditorBlueprintResources/StandardMacros.IncrementInt` (`self.WeldState`))))
          (:`1`
            (if (>= (`self.CurrentWeldTime`) (* (`self.TargetWeldTime`) 0.66))
              (`StaticMeshComponent.SetStaticMesh` (`self.CrackState`) (`self.CrackStateSmall`))
              (`/Engine/EditorBlueprintResources/StandardMacros.IncrementInt` (`self.WeldState`))))
          (:`2`
            (if (>= (`self.CurrentWeldTime`) (`self.TargetWeldTime`))
              (`SceneComponent.SetVisibility` (`self.CrackState`) false false)
              (`AudioComponent.Stop` (`self.WeldSound`))
              (`self.Fix`)
              (`self.ExitTask`)))))))
  (:`Started`
    ;[1 1 1] start weld
    (set `self.CurrentWeldTime` 0.0)
    (`|ExecutionSequence`
      (:`then_0`
        (bind _returnvalue (`GameplayStatics.SpawnSound2D` (`/Game/Blueprints/Tools/BP_Tool.RepairSound` _equippedtool) 1.0 1.0 0.0 null))
        (set `self.WeldSound` _returnvalue)
        (set `/Game/Blueprints/Tools/BP_Tool.TargetSceneComponent` (`self.ToolSocket`) (`/Game/Blueprints/BP_Character.EquippedTool` (`self.Character Ref`))))
      (:`then_1`
        (bind _asbp_welder (cast `/Game/Blueprints/Tools/BP_Welder` _equippedtool))
        (`/Game/Blueprints/Tools/BP_Welder.StartWelding` _asbp_welder))))
  (:`Completed`
    (`AudioComponent.Stop` (`self.WeldSound`))
    (bind _asbp_welder_2 (cast `/Game/Blueprints/Tools/BP_Welder` (`/Game/Blueprints/BP_Character.EquippedTool` (`self.Character Ref`))))
    (`/Game/Blueprints/Tools/BP_Welder.StopWelding` _asbp_welder_2)))

(event `self.ExitTask`
  (`AudioComponent.Stop` (`self.WeldSound`))
  (bind _asbp_welder (cast `/Game/Blueprints/Tools/BP_Welder` (`/Game/Blueprints/BP_Character.EquippedTool` (`self.Character Ref`))))
  (`/Game/Blueprints/Tools/BP_Welder.StopWelding` _asbp_welder)
  (`parent.ExitTask`))

(fn `UserConstructionScript`
  (`parent.UserConstructionScript`)
  (`StaticMeshComponent.SetStaticMesh` (`self.CrackState`) (`self.CrackStateLarge`)))