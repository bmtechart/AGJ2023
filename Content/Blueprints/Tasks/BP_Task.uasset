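; Possessable repair task that starts broken and steadily raises the game mode's WaterLevel until fixed.
; Interacting with the required tool equipped blends the camera to the task, possesses it, swaps Enhanced Input mapping contexts and hides the HUD.
; Fix clears the broken state and stops audio.
; ExitTask separately restores the character's possession, input, HUD and tool attachment target, using delays timed to the camera blend.
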(event `self.ReceiveBeginPlay`
  ;[0 0.1693 1 1 50] BEGIN PLAY
  (bind _asbp_main_game_mode (cast `/Game/Blueprints/BP_MainGameMode` (`GameplayStatics.GetGameMode`)))
  (set `self.MainGameMode` _asbp_main_game_mode)
  (`self.Break`))

(event `self.ReceiveTick`
  (params (DeltaSeconds :type "Float (single-precision)"))
  ;[1 0 0 1 50] TICK
  ;;[1 1 1] if broken, slowly add to water level
  (if (`self.bIsBroken`)
    (set `/Game/Blueprints/BP_MainGameMode.WaterLevel` (+ (* DeltaSeconds (`self.FillRate`)) (`/Game/Blueprints/BP_MainGameMode.WaterLevel` (`self.MainGameMode`))) (`self.MainGameMode`))))

(event `/Game/Blueprints/BPI_Interactable.Interact`
  (params (CharacterRef :type "/Game/Blueprints/BP_Character Object Reference"))
  (bind _equippedtool (`/Game/Blueprints/BP_Character.EquippedTool` CharacterRef))
  ;[0 1 0.1754 1 50] INTERACT EVENT
  (set `self.Character Ref` CharacterRef)
  (if (`self.bIsBroken`)
    (`/Engine/EditorBlueprintResources/StandardMacros.IsValid` _equippedtool
      (:`Is Valid`
        (if (`|EnumEquality` (`/Game/Blueprints/Tools/BP_Tool.ToolType` _equippedtool) (`self.ToolRequired`))
          (`self.EnterTask`))))))

(event `Fix`
  ;[1 1 1] FIX
  (set `self.bIsBroken` false)
  (`AudioComponent.Stop` (`self.Audio`)))

(event `Break`
  ;[1 1 1] Break
  (set `self.bIsBroken` true)
  (`GameplayStatics.PlaySoundAtLocation` (`AudioComponent.Sound` (`self.Audio`)) (`self.K2_GetActorLocation`) (struct) 1.0 1.0 0.0 null null null null))

(event `EnterTask`
  ;[1 1 1 1 50] Transition to task state
  (`EnhancedInputSubsystemInterface.RemoveMappingContext` (pcsubsystem `EnhancedInputLocalPlayerSubsystem` (`GameplayStatics.GetPlayerController` 0)) "/Game/Input/PlayerMovement/IMC_PlayerInput.IMC_PlayerInput" (struct))
  (`PlayerController.SetViewTargetWithBlend` (`GameplayStatics.GetPlayerController` 0) self (`self.TaskTransitionBlendTime`) "VTBlend_Linear" 0.0 true)
  (`KismetSystemLibrary.Delay` (+ (`self.TaskTransitionBlendTime`) 0.1))
  (`Controller.Possess` (`GameplayStatics.GetPlayerController` 0) self)
  (`EnhancedInputSubsystemInterface.AddMappingContext` (pcsubsystem `EnhancedInputLocalPlayerSubsystem` (`GameplayStatics.GetPlayerController` 0)) (`self.TaskInputMappingContext`) 0 (struct))
  (`Widget.SetVisibility` (`/Game/Blueprints/BP_Character.PlayerHUD` (`self.Character Ref`)) "Hidden"))

(event `ExitTask`
  (bind _returnvalue (`GameplayStatics.GetPlayerController` 0))
  (bind _returnvalue_2 (`GameplayStatics.GetPlayerController` 0))
  (bind _character_ref (`self.Character Ref`))
  ;[1 1 1 1 50] Exit Task
  (`Controller.UnPossess` (`GameplayStatics.GetPlayerController` 0))
  (`PlayerController.SetViewTargetWithBlend` (`GameplayStatics.GetPlayerController` 0) (`self.Character Ref`) (`self.TaskTransitionBlendTime`) "VTBlend_Linear" 0.0 true)
  (`EnhancedInputSubsystemInterface.RemoveMappingContext` (pcsubsystem `EnhancedInputLocalPlayerSubsystem` (`GameplayStatics.GetPlayerController` 0)) (`self.TaskInputMappingContext`) (struct))
  (`KismetSystemLibrary.Delay` (+ (`self.TaskTransitionBlendTime`) 0.1))
  (`Widget.SetVisibility` (`/Game/Blueprints/BP_Character.PlayerHUD` (`self.Character Ref`)) "Visible")
  (set `PlayerController.bShowMouseCursor` false _returnvalue_2)
  (`WidgetBlueprintLibrary.SetInputMode_GameOnly` _returnvalue_2)
  (set `/Game/Blueprints/Tools/BP_Tool.TargetSceneComponent` (`/Game/Blueprints/BP_Character.ToolSocket` _character_ref) (`/Game/Blueprints/BP_Character.EquippedTool` _character_ref))
  (`EnhancedInputSubsystemInterface.AddMappingContext` (pcsubsystem `EnhancedInputLocalPlayerSubsystem` (`GameplayStatics.GetPlayerController` 0)) "/Game/Input/PlayerMovement/IMC_PlayerInput.IMC_PlayerInput" 0 (struct))
  (`Controller.UnPossess` _returnvalue)
  (`Controller.Possess` _returnvalue (`self.Character Ref`)))

(fn `UserConstructionScript`)