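; BP_Pump is a breakable mechanic that drains water from the level while it is working.
; On Tick, unless broken, it lowers the WaterLevel value on BP_MainGameMode by PumpRate scaled by delta time.
; Break and Repair call the parent logic, then play 2D pump shutdown and startup cues.
; BeginPlay caches the game mode and a BP_WaterLevel actor, though that actor is not used in these graphs.
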(event `self.Break`
  (`parent.Break`)
  (`GameplayStatics.PlaySound2D` "/Game/Audio/SFX/Pump/PumpKeep2Off_Cue.PumpKeep2Off_Cue" 0.5 1.0 0.0 null null))

(event `self.Repair`
  (`parent.Repair`)
  (`GameplayStatics.PlaySound2D` "/Game/Audio/SFX/Pump/PumpOn2Keep_Cue.PumpOn2Keep_Cue" 0.5 1.0 0.0 null null))

(event `self.ReceiveBeginPlay`
  (bind _returnvalue (`GameplayStatics.GetActorOfClass` "/Game/Blueprints/BP_WaterLevel.BP_WaterLevel_C"))
  (set `self.WaterLevel` _returnvalue)
  (bind _asbp_main_game_mode (cast `/Game/Blueprints/BP_MainGameMode` (`GameplayStatics.GetGameMode`)))
  (set `self.MainGameMode_0` _asbp_main_game_mode))

(event `self.ReceiveTick`
  (params (DeltaSeconds :type "Float (single-precision)"))
  (if (not (`self.bIsBroken`))
    (set `/Game/Blueprints/BP_MainGameMode.WaterLevel` (- (`/Game/Blueprints/BP_MainGameMode.WaterLevel` (`self.MainGameMode_0`)) (* DeltaSeconds (`self.PumpRate`))) (`self.MainGameMode_0`))))

(event `/Game/Blueprints/BPI_Interactable.Interact`
  (params (CharacterRef :type "/Game/Blueprints/BP_Character Object Reference")))

(fn `UserConstructionScript`)