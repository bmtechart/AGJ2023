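; BP_WarningLight is a rotating warning light actor built around two spotlights.
; Tick spins both spotlights around their relative yaw at RotationRate, scaled by delta time, whether or not they are lit.
; TurnOn and TurnOff events switch the light by setting both intensities to a fixed brightness or zero; nothing in this graph calls them.
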(event `self.ReceiveTick`
  (params (DeltaSeconds :type "Float (single-precision)"))
  (bind _returnvalue (* DeltaSeconds (`self.RotationRate`)))
  (`SceneComponent.K2_AddRelativeRotation` (`self.SpotLight`) (`KismetMathLibrary.MakeRotator` 0.0 0.0 _returnvalue) false false)
  (`SceneComponent.K2_AddRelativeRotation` (`self.SpotLight1`) (`KismetMathLibrary.MakeRotator` 0.0 0.0 _returnvalue) false false))

(event `TurnOn`
  (`LightComponent.SetIntensity` (`self.SpotLight`) 3000.0)
  (`LightComponent.SetIntensity` (`self.SpotLight1`) 3000.0))

(event `TurnOff`
  (`LightComponent.SetIntensity` (`self.SpotLight`) 0.0)
  (`LightComponent.SetIntensity` (`self.SpotLight1`) 0.0))

(fn `UserConstructionScript`)