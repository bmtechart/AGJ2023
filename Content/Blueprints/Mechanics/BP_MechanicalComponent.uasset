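; BP_MechanicalComponent is a repairable mechanical component whose broken state follows a set of composite tasks and is shown by a warning light.
; The construction script binds events to each task's broken and fixed notifications.
; Break and Repair set the broken flag and switch the light.
; CheckRepair, run at BeginPlay, scans the tasks and calls Repair only when none is found broken.
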(event `self.ReceiveBeginPlay`
  (`self.CheckRepair`))

(event `Repair`
  (set `self.bIsBroken` false)
  (`/Game/Blueprints/Mechanics/BP_WarningLight.TurnOff` (`self.WarningLight`)))

(event `Break`
  (set `self.bIsBroken` true)
  (`/Game/Blueprints/Mechanics/BP_WarningLight.TurnOn` (`self.WarningLight`)))

(event `CheckRepair`
  (for _array_element (`self.CompositeTasks`)
    (set `self.bIsBroken` false)
    (if (`/Game/Blueprints/Tasks/BP_Task.bIsBroken` _array_element)
      (set `self.bIsBroken` true)
      (break)))
  (if (not (`self.bIsBroken`))
    (`self.Repair`)))

(fn `UserConstructionScript`
  (for _array_element (`self.CompositeTasks`)
    (add `/Game/Blueprints/Tasks/BP_Task.TaskBroken` _array_element (`|CreateDelegate` :!event `Break`))
    (add `/Game/Blueprints/Tasks/BP_Task.TaskFixed` _array_element (`|CreateDelegate` :!event `CheckRepair`))))