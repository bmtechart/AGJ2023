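; First-person player character that moves, looks, interacts with objects and carries one tool at a time.
; BeginPlay adds the Enhanced Input mapping and HUD, while Tick line-traces the looked-at actor and feeds the socket position to the held tool.
; Camera sphere traces on separate channels send BPI_Interactable messages or grab a BP_Tool.
; Equip drops any current tool back into physics and sets the new one interpolating toward the socket instead of attaching it.
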(event `self.ReceiveTick`
  (params (DeltaSeconds :type "Float (single-precision)"))
  (bind _camera (`self.Camera`))
  (bind _equippedtool (`self.EquippedTool`))
  (bind _returnvalue (`SceneComponent.K2_GetComponentLocation` _camera))
  ;[1 1 1] Tick
  (`|ExecutionSequence`
    (:`then_0`
      ;[1 1 1] What actor are we looking at?
      (bind _outhit (`KismetSystemLibrary.LineTraceSingle` _returnvalue (+ _returnvalue (* (`SceneComponent.GetForwardVector` _camera) (`self.InteractionRange`))) "TraceTypeQuery1"))
      (set `self.LookAtActor` (`.HitActor` (`GameplayStatics.BreakHitResult` _outhit))))
    (:`then_1`
      (`/Engine/EditorBlueprintResources/StandardMacros.IsValid` _equippedtool
        (:`Is Valid`
          (set `/Game/Blueprints/Tools/BP_Tool.TargetPosition` (`SceneComponent.K2_GetComponentLocation` (`self.ToolSocket`)) _equippedtool))))))

(event `self.ReceiveBeginPlay`
  ;[1 1 1] Begin Play
  ;;[1 1 1] map player inputs
  (`EnhancedInputSubsystemInterface.AddMappingContext` (pcsubsystem `EnhancedInputLocalPlayerSubsystem` (`GameplayStatics.GetPlayerController` 0)) "/Game/Input/PlayerMovement/IMC_PlayerInput.IMC_PlayerInput" 0 (struct))
  ;;[1 1 1] Add UI
  (`/Engine/EditorBlueprintResources/StandardMacros.IsValid` (`self.PlayerHUD`)
    (:`Is Valid`
      _)
    (:`Is Not Valid`
      (bind _returnvalue (`|CreateWidget` "/Game/UI/WBP_GameUI.WBP_GameUI_C" null self))
      (set `self.PlayerHUD` _returnvalue)))
  (`UserWidget.AddToViewport` (`self.PlayerHUD`) 0))

(event `EnhancedInput|/Game/Input/PlayerMovement/IA_Move`
  (params (ActionValue :type "Vector2D Structure") (ElapsedSeconds :type "Float (double-precision)") (TriggeredSeconds :type "Float (double-precision)") (InputAction :type "InputAction Object Reference" :default "/Game/Input/PlayerMovement/IA_Move.IA_Move"))
  ;[0.4606 0 1 1 50] IA MOVEMENT
  (:`Triggered`
    (`self.AddMovementInput` (`self.GetActorRightVector`) ActionValue_X)
    (`self.AddMovementInput` (`self.GetActorForwardVector`) ActionValue_Y)))

(event `EnhancedInput|/Game/Input/PlayerMovement/IA_Look`
  (params (ActionValue :type "Vector2D Structure") (ElapsedSeconds :type "Float (double-precision)") (TriggeredSeconds :type "Float (double-precision)") (InputAction :type "InputAction Object Reference" :default "/Game/Input/PlayerMovement/IA_Look.IA_Look"))
  ;[0.5427 1 0 1 50] IA LOOK
  (:`Triggered`
    (`self.AddControllerYawInput` (* ActionValue_X -1.0))
    (`self.AddControllerPitchInput` ActionValue_Y)))

(event `EnhancedInput|/Game/Input/PlayerMovement/IA_Interact`
  (params (ActionValue :type Boolean) (ElapsedSeconds :type "Float (double-precision)") (TriggeredSeconds :type "Float (double-precision)") (InputAction :type "InputAction Object Reference" :default "/Game/Input/PlayerMovement/IA_Interact.IA_Interact"))
  (bind _camera (`self.Camera`))
  (bind _returnvalue (`SceneComponent.K2_GetComponentLocation` _camera))
  ;[0 1 0.9459 1 50] IA_Interact
  (:`Started`
    (bind (_outhit _returnvalue_2) (`KismetSystemLibrary.SphereTraceSingle` :`Start` _returnvalue :`End` (+ _returnvalue (* (`SceneComponent.GetForwardVector` _camera) (`self.InteractionRange`))) :`Radius` 100.0 :`TraceChannel` "TraceTypeQuery3" :`bTraceComplex` true :`DrawDebugType` "ForDuration"))
    (if _returnvalue_2
      (bind (_bblockinghit _binitialoverlap _time _distance _location _impactpoint _normal _impactnormal _physmat _hitactor) (`GameplayStatics.BreakHitResult` _outhit))
      (if (`KismetSystemLibrary.DoesImplementInterface` _hitactor "/Game/Blueprints/BPI_Interactable.BPI_Interactable_C")
        (message `/Game/Blueprints/BPI_Interactable.Interact` _hitactor self)))))

(event `EnhancedInput|/Game/Input/PlayerMovement/IA_Grab`
  (params (ActionValue :type Boolean) (ElapsedSeconds :type "Float (double-precision)") (TriggeredSeconds :type "Float (double-precision)") (InputAction :type "InputAction Object Reference" :default "/Game/Input/PlayerMovement/IA_Grab.IA_Grab"))
  (bind _camera (`self.Camera`))
  (bind _returnvalue (`SceneComponent.K2_GetComponentLocation` _camera))
  ;[1 1 1 1 50] IA_Equip
  (:`Started`
    (bind _outhit (`KismetSystemLibrary.SphereTraceSingle` :`Start` _returnvalue :`End` (+ _returnvalue (* (`SceneComponent.GetForwardVector` _camera) (`self.InteractionRange`))) :`Radius` 10.0 :`TraceChannel` "TraceTypeQuery4" :`bTraceComplex` true :`DrawDebugType` "ForDuration"))
    (bind _asbp_tool (cast `/Game/Blueprints/Tools/BP_Tool` (`.HitActor` (`GameplayStatics.BreakHitResult` _outhit))))
    (`self.Equip` _asbp_tool)))

(fn `Equip`
  (params (Tool :type "/Game/Blueprints/Tools/BP_Tool Object Reference"))
  (locals (InputTool :type "/Game/Blueprints/Tools/BP_Tool Object Reference"))
  (bind _equippedtool (`self.EquippedTool`))
  (bind _equippedtool_2 (`self.EquippedTool`))
  (bind _equippedtool_3 (`self.EquippedTool`))
  (set `local.InputTool` Tool)
  (`/Engine/EditorBlueprintResources/StandardMacros.IsValid` (`self.EquippedTool`)
    (:`Is Valid`
      ;[1 1 1] DropCurrentTool
      (`self.K2_DetachFromActor` (`self.EquippedTool`) "KeepWorld" "KeepWorld" "KeepWorld")
      (set `/Game/Blueprints/Tools/BP_Tool.InterpToPoint` false _equippedtool)
      (`PrimitiveComponent.SetSimulatePhysics` (`/Game/Blueprints/Tools/BP_Tool.Capsule` _equippedtool) true)
      (`PrimitiveComponent.SetCollisionResponseToChannel` (`/Game/Blueprints/Tools/BP_Tool.Capsule` (`self.EquippedTool`)) "ECC_GameTraceChannel2" "ECR_Block")
      (`PrimitiveComponent.SetCollisionEnabled` (`/Game/Blueprints/Tools/BP_Tool.Capsule` (`self.EquippedTool`)) "QueryAndPhysics"))
    (:`Is Not Valid`
      _))
  (set `self.EquippedTool` (`local.InputTool`))
  (`PrimitiveComponent.SetSimulatePhysics` (`/Game/Blueprints/Tools/BP_Tool.Capsule` _equippedtool_3) false)
  (set `/Game/Blueprints/Tools/BP_Tool.InterpToPoint` true _equippedtool_3)
  (`PrimitiveComponent.SetCollisionResponseToChannel` (`/Game/Blueprints/Tools/BP_Tool.Capsule` _equippedtool_2) "ECC_GameTraceChannel2" "ECR_Ignore")
  (`KismetSystemLibrary.PrintString` (`KismetStringLibrary.Concat_StrStr` "Equipped " (`|GetEnumeratorNameAsString` (`/Game/Blueprints/Tools/BP_Tool.ToolType` _equippedtool_2)))))

(fn `UserConstructionScript`)