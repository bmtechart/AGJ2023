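; BP_Task is an interactable task actor, such as a leak, that raises the level's water while it is broken.
; On BeginPlay it finds the BP_WaterLevel actor and starts broken, adding FillRate scaled by delta time to that actor's WaterLevel every tick.
; Interact prints a fixed message, deactivates the Niagara effect and clears the broken flag, which stops the filling.
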(event `self.ReceiveBeginPlay`
  (bind _returnvalue (`GameplayStatics.GetActorOfClass` "/Game/Blueprints/BP_WaterLevel.BP_WaterLevel_C"))
  (set `self.WaterLevelActor` _returnvalue)
  (set `self.bIsBroken` true))

(event `self.ReceiveTick`
  (params (DeltaSeconds :type "Float (single-precision)"))
  (bind _waterlevelactor (`self.WaterLevelActor`))
  ;[1 1 1] TICK
  (if (`self.bIsBroken`)
    (set `/Game/Blueprints/BP_WaterLevel.WaterLevel` (+ (* (`self.FillRate`) DeltaSeconds) (`/Game/Blueprints/BP_WaterLevel.WaterLevel` _waterlevelactor)) _waterlevelactor)))

(event `/Game/Blueprints/BPI_Interactable.Interact`
  ;[1 1 1] Comment
  (`KismetSystemLibrary.PrintString` (`KismetStringLibrary.Concat_StrStr` (`KismetSystemLibrary.GetDisplayName` self) " fixed!"))
  (`ActorComponent.Deactivate` (`self.Niagara`))
  (set `self.bIsBroken` false))

(fn `UserConstructionScript`)