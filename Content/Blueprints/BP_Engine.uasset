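; BP_Engine is an engine that drives the game's depth, with separate rates for working and broken states.
; On BeginPlay it casts and caches BP_MainGameMode.
; Each Tick it calls AdjustDepth on the game mode with LiftRate while intact or DiveRate while IsBroken, scaled by delta time.
; Break and Fix events are empty here, so this graph only reads the broken flag.
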(event `self.ReceiveBeginPlay`
  (bind _asbp_main_game_mode (cast `/Game/Blueprints/BP_MainGameMode` (`GameplayStatics.GetGameMode`)))
  (set `self.MainGameMode` _asbp_main_game_mode))

(event `self.ReceiveTick`
  (params (DeltaSeconds :type "Float (single-precision)"))
  (if (not (`self.bIsBroken`))
    (`/Game/Blueprints/BP_MainGameMode.AdjustDepth` (`self.MainGameMode`) (* DeltaSeconds (`self.LiftRate`)))
    (else
      (`/Game/Blueprints/BP_MainGameMode.AdjustDepth` (`self.MainGameMode`) (* DeltaSeconds (`self.DiveRate`))))))

(event `Break`)

(event `Fix`)

(fn `UserConstructionScript`)