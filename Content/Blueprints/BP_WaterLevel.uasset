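; Water level actor that positions a water component between a bottom and a top marker.
; Every Tick calls SetWaterLevel, which lerps WaterParent's world location between WaterBottom and WaterTop using the WaterLevel alpha.
; WaterLevel resets to empty on BeginPlay and is not changed afterward within this Blueprint.
; The Tick check for a full level has no action attached.
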(event `self.ReceiveBeginPlay`
  (set `self.WaterLevel` 0.0))

(event `self.ReceiveTick`
  (params (DeltaSeconds :type "Float (single-precision)"))
  (`self.SetWaterLevel`)
  (if (>= (`self.WaterLevel`) 1.0)
    _))

(fn `SetWaterLevel`
  (`SceneComponent.K2_SetWorldLocation` (`self.WaterParent`) (`KismetMathLibrary.VLerp` (`SceneComponent.K2_GetComponentLocation` (`self.WaterBottom`)) (`SceneComponent.K2_GetComponentLocation` (`self.WaterTop`)) (`self.WaterLevel`)) false false))

(fn `UserConstructionScript`)