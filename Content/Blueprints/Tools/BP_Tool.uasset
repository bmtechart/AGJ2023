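; BP_Tool is a tool actor whose ToolPoint component follows a target scene component and which plays a sound when used for repair.
; Each Tick, if the target is valid, it moves ToolPoint with VInterpTo at PositionInterpSpeed and rotates it with RInterpTo, which has no speed set.
; Repair only plays a 2D sound, Interact is empty, and an alternative that moves the whole actor is left unconnected.
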(event `self.ReceiveTick`
  (params (DeltaSeconds :type "Float (single-precision)"))
  (bind _toolpoint (`self.ToolPoint`))
  (`/Engine/EditorBlueprintResources/StandardMacros.IsValid` (`self.TargetSceneComponent`)
    (:`Is Valid`
      (`SceneComponent.K2_SetWorldLocation` _toolpoint (`KismetMathLibrary.VInterpTo` (`SceneComponent.K2_GetComponentLocation` _toolpoint) (`SceneComponent.K2_GetComponentLocation` (`self.TargetSceneComponent`)) (`GameplayStatics.GetWorldDeltaSeconds`) (`self.PositionInterpSpeed`)) false false)
      (`SceneComponent.K2_SetWorldRotation` _toolpoint (`KismetMathLibrary.RInterpTo` (`SceneComponent.K2_GetComponentRotation` _toolpoint) (`SceneComponent.K2_GetComponentRotation` (`self.TargetSceneComponent`)) (`GameplayStatics.GetWorldDeltaSeconds`)) false false))))

(event `/Game/Blueprints/BPI_Interactable.Interact`
  (params (CharacterRef :type "/Game/Blueprints/BP_Character Object Reference")))

(event `Repair`
  (`GameplayStatics.PlaySound2D` (`self.RepairSound`) 1.0 1.0 0.0 null null))

(fn `UserConstructionScript`)